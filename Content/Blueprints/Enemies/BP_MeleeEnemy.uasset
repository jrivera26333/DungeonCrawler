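; Melee enemy Blueprint that sets its starting health on BeginPlay and reacts to damage and death.
; An interface event for damage taken plays a hit sound at the enemy's location.
; An interface event for death sets the IsDead flag and disables capsule collision.
; The construction script only calls its parent, and the graphs shown contain no attack or movement logic.
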(event `self.ReceiveBeginPlay`
  (`self.SetHealth` 100.0))

(event `/Game/Blueprints/Interfaces/HealthInterface.OnDamageTaken`
  ;[1 0.8931 0] On Damage Taken Interface
  (`GameplayStatics.PlaySoundAtLocation` (`self.HitSound`) (`self.K2_GetActorLocation`) (struct) 1.0 1.0 0.0 null null null null))

(event `/Game/Blueprints/Interfaces/HealthInterface.OnDeath`
  ;[0 0 0] On Death Interface
  (set `self.IsDead` true)
  (`PrimitiveComponent.SetCollisionEnabled` (`self.CapsuleComponent`) "NoCollision"))

(fn `UserConstructionScript`
  (`parent.UserConstructionScript`))