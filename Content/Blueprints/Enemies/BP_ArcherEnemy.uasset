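; Archer enemy Blueprint that carries a bow, fires arrows, shows a health bar and drops loot on death.
; BeginPlay sets health, caches the health widget and attaches a spawned bow to a hand socket with physics off.
; RangeAttack plays a montage, while a separate SpawnArrow event spawns arrows at ArrowPlacement.
; Damage updates the bar and plays a sound; death disables capsule collision, hides the bar and launches physics-driven loot with random impulse.
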(event `self.ReceiveBeginPlay`
  (`self.SetHealth` 100.0)
  ;[1 1 1] Creating Enemy Weapon on Start
  (`self.CreateEnemyHealthWidget`)
  (bind _returnvalue (`|SpawnActorFromClass` "/Game/Blueprints/Props/BP_Bow.BP_Bow_C" (`self.GetTransform`) "Undefined" "OverrideRootScale" null null))
  (`self.K2_AttachToComponent` _returnvalue (`self.Mesh`) "armBowLeftSocket" "SnapToTarget" "SnapToTarget" "KeepWorld" true)
  (bind _capsulecollider (`/Game/Blueprints/Props/BP_InteractObject.GetCollider` _returnvalue))
  (`PrimitiveComponent.SetSimulatePhysics` _capsulecollider false)
  (`PrimitiveComponent.SetEnableGravity` _capsulecollider false)
  (set `self.CombatHandedWeapon` _returnvalue))

(event `/Game/Blueprints/Interfaces/HealthInterface.OnDamageTaken`
  ;[1 0.8931 0] On Damage Taken Interface
  (set `/Game/Blueprints/UI/WBP_AIHealth.Health` (`self.GetHealth`) (`self.HealthWidgetRef`))
  (`GameplayStatics.PlaySoundAtLocation` (`self.HitSound`) (`self.K2_GetActorLocation`) (struct) 1.0 1.0 0.0 null null null null))

(event `/Game/Blueprints/Interfaces/HealthInterface.OnDeath`
  ;[1 1 1] Binding to OnDeath
  (`self.SetIsDead` true)
  (`PrimitiveComponent.SetCollisionEnabled` (`self.CapsuleComponent`) "NoCollision")
  (`self.SpawnLoot`)
  (bind _aswbp_aihealth (cast `/Game/Blueprints/UI/WBP_AIHealth` (`WidgetComponent.GetWidget` (`self.HealthWidget`))))
  (`/Game/Blueprints/UI/WBP_AIHealth.HideHealthBar` _aswbp_aihealth))

(event `RangeAttack`
  (`self.PlayAnimMontage` null))

(event `SpawnArrow`
  (`|SpawnActorFromClass` "/Game/Blueprints/Props/BP_Arrow.BP_Arrow_C" (`SceneComponent.K2_GetComponentToWorld` (`self.ArrowPlacement`)) "Undefined" "OverrideRootScale" null null)
  (`KismetSystemLibrary.PrintString` "Called"))

(fn `CreateEnemyHealthWidget`
  (bind _aswbp_aihealth (cast `/Game/Blueprints/UI/WBP_AIHealth` (`WidgetComponent.GetUserWidgetObject` (`self.HealthWidget`))))
  (bind _output_get (set `self.HealthWidgetRef` _aswbp_aihealth))
  (set `/Game/Blueprints/UI/WBP_AIHealth.Health` 100.0 _output_get))

(fn `SpawnLoot`
  (locals (SpawnedActor :type "/Game/Blueprints/Props/BP_Equipable Object Reference"))
  (bind _returnvalue (`KismetMathLibrary.RandomFloatInRange` 250.0 500.0))
  (bind _returnvalue_2 (`KismetMathLibrary.MakeVector` _returnvalue _returnvalue (`KismetMathLibrary.RandomFloatInRange` 2500.0 4000.0)))
  (bind _returnvalue_3 (`|SpawnActorFromClass` (`self.LootToSpawn`) (`self.GetTransform`) "Undefined" "OverrideRootScale" null null))
  (bind _output_get (set `local.SpawnedActor` _returnvalue_3))
  (bind _capsulecollider (`/Game/Blueprints/Props/BP_InteractObject.GetCollider` _output_get))
  (`PrimitiveComponent.SetEnableGravity` _capsulecollider true)
  (`PrimitiveComponent.SetSimulatePhysics` _capsulecollider true)
  (`PrimitiveComponent.AddImpulse` _capsulecollider _returnvalue_2 "None" false)
  (`SceneComponent.K2_AddLocalRotation` _capsulecollider (`KismetMathLibrary.Conv_VectorToRotator` _returnvalue_2) false false))

(fn `UserConstructionScript`
  (`parent.UserConstructionScript`))