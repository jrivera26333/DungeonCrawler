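; BP_Bow is a bow prop Blueprint that marks itself as left-handed and supplies its interaction name and attach socket.
; On BeginPlay it calls the parent and sets the left-handed flag to true.
; It overrides parent functions to return "Bow" as the interaction name and the left-arm bow socket as its socket position.
; Overlap and tick events are unused, and other behavior comes from the parent class.
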(event `self.ReceiveBeginPlay`
  (`parent.ReceiveBeginPlay`)
  (`self.SetIsLeftHanded` true))

(fn `GetInteractionName`
  (returns (HoveredActor :type Text))
  (return "Bow"))

(fn `GetSocketPosition`
  (returns (SocketName :type Name))
  (return "armBowLeftSocket"))

(fn `SetIsLeftHanded`
  (params (IsLeftHanded :type Boolean))
  (`parent.SetIsLeftHanded` IsLeftHanded))

(fn `UserConstructionScript`
  (`parent.UserConstructionScript`))