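; One-handed weapon prop that attaches itself to the player's BP_MainCharacter when picked up.
; BeginPlay caches the character, then Pickup chooses the left or right arm socket from IsLeftHandedItem.
; If that hand is empty, it snaps to the socket keeping world scale and registers as the held item.
; GetWeaponMesh exposes the static mesh, while detach and rescale nodes are left unconnected.
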(event `self.ReceiveBeginPlay`
  (bind _asbp_main_character (cast `/Game/Blueprints/Character/BP_MainCharacter` (`GameplayStatics.GetPlayerCharacter` 0)))
  (set `self.MainCharacter` _asbp_main_character))

(event `/Game/Blueprints/Interfaces/WeaponInterface.Pickup`
  (bind _maincharacter (`self.MainCharacter`))
  (`/Engine/EditorBlueprintResources/StandardMacros.IsValid` (`self.MainCharacter`)
    (:`Is Valid`
      (if (`self.IsLeftHandedItem`)
        (set `self.CharacterWeaponSocket` "armLeftSocket")
        (`/Engine/EditorBlueprintResources/StandardMacros.IsValid` (`/Game/Blueprints/Character/BP_MainCharacter.GetLeftHeldItem` (`self.MainCharacter`))
          (:`Is Not Valid`
            _))
        (else
          (set `self.CharacterWeaponSocket` "armRightSocket")
          (`/Engine/EditorBlueprintResources/StandardMacros.IsValid` (`/Game/Blueprints/Character/BP_MainCharacter.GetRightHeldItem` (`self.MainCharacter`))
            (:`Is Not Valid`
              _))))
      (`self.K2_AttachToComponent` (`Character.Mesh` (`self.MainCharacter`)) (`self.CharacterWeaponSocket`) "SnapToTarget" "SnapToTarget" "KeepWorld")
      (if (`self.IsLeftHandedItem`)
        (`/Game/Blueprints/Character/BP_MainCharacter.SetLeftHeldItem` _maincharacter self)
        (else
          (`/Game/Blueprints/Character/BP_MainCharacter.SetRightHeldItem` _maincharacter self))))))

(fn `GetWeaponMesh`
  (returns (WeaponMesh :type "StaticMeshComponent Object Reference"))
  (return (`self.StaticMesh`)))

(fn `UserConstructionScript`)