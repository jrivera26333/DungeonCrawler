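; BP_Equipment is an equippable item that attaches to the player character's left or right hand, with the player cached on BeginPlay.
; Equip picks the arm socket from IsLeftHandedItem and proceeds only if that hand is empty.
; It then disables Box physics and gravity, attaches to the character mesh, registers itself as held, and plays a sound and particle effect.
; GetWeaponMesh exposes the static mesh, while Swap is an empty stub.
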(event `self.ReceiveBeginPlay`
  (bind _asbp_base_character (cast `/Game/Blueprints/Character/BP_BaseCharacter` (`GameplayStatics.GetPlayerCharacter` 0)))
  (set `self.MainCharacter` _asbp_base_character))

(fn `Equip`
  (bind _maincharacter (`self.MainCharacter`))
  (bind _box (`self.Box`))
  (`/Engine/EditorBlueprintResources/StandardMacros.IsValid` (`self.MainCharacter`)
    (:`Is Valid`
      (if (`self.IsLeftHandedItem`)
        (set `self.CharacterWeaponSocket` "armLeftSocket")
        (`/Engine/EditorBlueprintResources/StandardMacros.IsValid` (`/Game/Blueprints/Character/BP_BaseCharacter.GetLeftHeldItem` (`self.MainCharacter`))
          (:`Is Not Valid`
            _))
        (else
          (set `self.CharacterWeaponSocket` "armRightSocket")
          (`/Engine/EditorBlueprintResources/StandardMacros.IsValid` (`/Game/Blueprints/Character/BP_BaseCharacter.GetRightHeldItem` (`self.MainCharacter`))
            (:`Is Not Valid`
              _))))
      (`PrimitiveComponent.SetSimulatePhysics` _box false)
      (`PrimitiveComponent.SetEnableGravity` _box false)
      (`self.K2_AttachToComponent` (`Character.Mesh` (`self.MainCharacter`)) (`self.CharacterWeaponSocket`) "SnapToTarget" "SnapToTarget" "KeepWorld")
      (if (`self.IsLeftHandedItem`)
        (`/Game/Blueprints/Character/BP_BaseCharacter.SetLeftHeldItem` _maincharacter self)
        (else
          (`/Game/Blueprints/Character/BP_BaseCharacter.SetRightHeldItem` _maincharacter self)))
      (`GameplayStatics.PlaySoundAtLocation` "/Game/Audio/Weapons/Sword_Equip_02.Sword_Equip_02" (0.0 0.0 0.0) (struct) 1.0 1.0 0.0 null null null null)
      (`NiagaraFunctionLibrary.SpawnSystemAtLocation` "/Game/Particles/PS_SwordHit.PS_SwordHit" (`self.K2_GetActorLocation`) (struct) (10.0 10.0 10.0)))))

(fn `GetWeaponMesh`
  (returns (WeaponMesh :type "StaticMeshComponent Object Reference"))
  (return (`self.StaticMesh`)))

(fn `Swap`
  (params (CurrentHeldWeapon :type "/Game/Blueprints/Props/BP_Equipment Object Reference")))

(fn `UserConstructionScript`)