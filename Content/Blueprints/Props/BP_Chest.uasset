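; BP_Chest is an interactable chest prop that opens its lid when a character interacts with it.
; ItemInteraction resets the character's current interactable, plays a sound at the chest's location and starts a timeline.
; Each timeline update adds local roll to ChestTop, scaled by the track value and OpenAngle, so rotation accumulates rather than being set absolutely.
; The same update calls DisableEvents.
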(event `/Game/Blueprints/Interfaces/InteractInterface.ItemInteraction`
  (params (Character :type "/Game/Blueprints/Character/BP_BaseCharacter Object Reference"))
  (`/Game/Blueprints/Character/BP_BaseCharacter.ResetCurrentInteractableObject` Character)
  (`self.PlayInteractionSound`)
  (bind (_direction _chest_animation_track) (`Timeline|Timeline_0`)
    (:`Update`
      (`SceneComponent.K2_AddLocalRotation` (`self.ChestTop`) (`KismetMathLibrary.MakeRotator` (* _chest_animation_track (`self.OpenAngle`))) false false)
      (`self.DisableEvents`))))

(fn `PlayInteractionSound`
  (`GameplayStatics.PlaySoundAtLocation` (`self.SoundInteraction`) (`self.K2_GetActorLocation`) (struct) 1.0 1.0 0.0 null null null null))

(fn `UserConstructionScript`)