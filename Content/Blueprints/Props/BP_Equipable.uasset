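; BP_Equipable is an equippable prop that the player picks up through interaction.
; Its ItemInteraction event passes the prop itself to the player character's EquipItem.
; Accessors expose its static mesh and a settable left-handed flag.
; The interaction name and socket position getters return only empty and None placeholders.
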(event `self.ReceiveBeginPlay`
  (`parent.ReceiveBeginPlay`))

(event `/Game/Blueprints/Interfaces/InteractInterface.ItemInteraction`
  (params (PlayerCharacter :type "/Game/Blueprints/Character/BP_PlayerCharacter Object Reference"))
  ;[0 1 0.2687] Equip Item games usually click for item pickups
  (`/Game/Blueprints/Character/BP_BaseCharacter.EquipItem` PlayerCharacter self))

(fn `GetInteractionName`
  (returns (HoveredActor :type Text))
  (return ""))

(fn `GetIsLeftHanded`
  (returns (Return :type Boolean))
  (return (`self.IsLeftHanded`)))

(fn `GetMesh`
  (returns (Return :type "StaticMeshComponent Object Reference"))
  (return (`self.StaticMesh`)))

(fn `GetSocketPosition`
  (returns (SocketName :type Name))
  (return "None"))

(fn `SetIsLeftHanded`
  (params (IsLeftHanded :type Boolean))
  (set `self.IsLeftHanded` IsLeftHanded)
  (return))

(fn `UserConstructionScript`
  (`parent.UserConstructionScript`))