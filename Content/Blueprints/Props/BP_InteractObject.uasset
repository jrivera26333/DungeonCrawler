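; BP_InteractObject is a base Blueprint for interactable props, meant to be specialized by derived classes.
; It exposes its Capsule as the collider and stores a HasBeenInteracted flag behind a getter and setter.
; ItemInteraction only prints a not-implemented message and GetInteractionName returns an empty string, leaving both as placeholders for subclasses to override.
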(event `/Game/Blueprints/Interfaces/InteractInterface.ItemInteraction`
  (params (Character :type "/Game/Blueprints/Character/BP_BaseCharacter Object Reference"))
  (`KismetSystemLibrary.PrintString` "Has not been implemented by derived class"))

(fn `GetCollider`
  (returns (CapsuleCollider :type "CapsuleComponent Object Reference"))
  (return (`self.Capsule`)))

(fn `GetHasBeenInteracted`
  (returns (Return :type Boolean))
  (return (`self.HasBeenInteracted`)))

(fn `GetInteractionName`
  (returns (HoveredActor :type Text))
  (return ""))

(fn `SetHasBeenInteracted`
  (params (Return :type Boolean))
  (set `self.HasBeenInteracted` Return)
  (return))

(fn `UserConstructionScript`)