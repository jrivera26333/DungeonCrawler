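; BP_Collectable is a collectable prop Blueprint that tracks whether it has been acquired.
; It exposes a getter and setter for the HasBeenAquired flag and a helper that plays a valid interaction sound at the actor's location.
; SetIsInPlayerRange also writes HasBeenAquired rather than a separate range flag.
; The construction script is empty, and the graphs contain no overlap or pickup logic.
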(fn `GetHasBeenAquiredStatus`
  (returns (Return :type Boolean))
  (return (`self.HasBeenAquired`)))

(fn `PlayInteractionSound`
  (params (InteractionSound :type "SoundBase Object Reference"))
  (`/Engine/EditorBlueprintResources/StandardMacros.IsValid` InteractionSound
    (:`Is Valid`
      (`GameplayStatics.PlaySoundAtLocation` InteractionSound (`self.K2_GetActorLocation`) (struct) 1.0 1.0 0.0 null null null null))))

(fn `SetHasBeenAquiredStatus`
  (params (HasBeenAquired :type Boolean))
  (set `self.HasBeenAquired` HasBeenAquired)
  (return))

(fn `SetIsInPlayerRange`
  (params (HasBeenAquired :type Boolean))
  (set `self.HasBeenAquired` HasBeenAquired)
  (return))

(fn `UserConstructionScript`)