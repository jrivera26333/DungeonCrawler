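; Behavior tree task that picks a strafe destination for a BP_MeleeEnemy.
; A random coin flip offsets the mesh's world location either right and slightly forward, or left and slightly back, relative to the pawn's facing.
; It draws a debug line to that point, writes it to a blackboard vector key and finishes successfully, without any navigation or obstacle check.
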(event `self.ReceiveExecuteAI`
  (params (OwnerController :type "AIController Object Reference") (ControlledPawn :type "Pawn Object Reference"))
  (bind _returnvalue (`SceneComponent.K2_GetComponentLocation` (`Character.Mesh` (cast `/Game/Blueprints/Enemies/BP_MeleeEnemy` ControlledPawn :!pure true))))
  (bind _returnvalue_2 (`SceneComponent.K2_GetComponentLocation` (`Character.Mesh` (cast `/Game/Blueprints/Enemies/BP_MeleeEnemy` ControlledPawn :!pure true))))
  (bind _returnvalue_3 (+ _returnvalue (* (`Actor.GetActorForwardVector` ControlledPawn) -50.0) (* (`Actor.GetActorRightVector` ControlledPawn) -150.0)))
  (bind _returnvalue_4 (+ _returnvalue_2 (* (`Actor.GetActorForwardVector` ControlledPawn) 50.0) (* (`Actor.GetActorRightVector` ControlledPawn) 150.0)))
  (if (== (`KismetMathLibrary.RandomIntegerInRange` 0 1) 0)
    (`KismetSystemLibrary.DrawDebugLine` _returnvalue_2 _returnvalue_4)
    (`BTFunctionLibrary.SetBlackboardValueAsVector` (`self.BB_Ref`) _returnvalue_4)
    (else
      (`KismetSystemLibrary.DrawDebugLine` _returnvalue _returnvalue_3)
      (`BTFunctionLibrary.SetBlackboardValueAsVector` (`self.BB_Ref`) _returnvalue_3)))
  (`self.FinishExecute` true))